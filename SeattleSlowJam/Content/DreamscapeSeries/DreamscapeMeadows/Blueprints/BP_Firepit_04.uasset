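; Firepit prop with a flickering ambient light and a construction-time On switch.
; The construction script shows or hides Fire by the On flag and lowers Smoke when off.
; From BeginPlay, a randomly timed delay loop runs a macro that randomizes light intensity.
; Nested FlipFlops in the macro alternate orange shades and nudge the light's position, periodically resetting it to the location saved at start.
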(event `self.ReceiveBeginPlay`
  (set `self.Relative Location` (`SceneComponent.RelativeLocation` (`self.AmbientLight`)))
  (`KismetSystemLibrary.RetriggerableDelay` (`KismetMathLibrary.RandomFloatInRange` 0.3 0.1) :!label _label)
  (`self.NewMacro_0`
    (:`NewParam2`
      (goto _label))))

(fn `UserConstructionScript`
  (if (`self.On?`)
    (`SceneComponent.SetVisibility` (`self.Fire`) true false)
    (`SceneComponent.K2_AddRelativeLocation` (`self.Smoke`) (0.0 0.0 0.0) false true)
    (else
      (`SceneComponent.SetVisibility` (`self.Fire`) false false)
      (`SceneComponent.K2_AddRelativeLocation` (`self.Smoke`) (0.0 0.0 -40.0) false true))))