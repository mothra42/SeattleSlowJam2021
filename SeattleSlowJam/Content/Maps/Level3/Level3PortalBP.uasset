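; Level 3 portal actor with a ShrinkEvent that closes it.
; The event switches the Box to query-and-physics collision, then starts two timelines from the beginning in sequence.
; The first lerps an armchair into position while shrinking the Portal mesh to zero scale and fading its point light out; the second slides the other armchair to the opposite side.
; Each lerp starts from the current value, not a cached start.
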(event `ShrinkEvent`
  (bind _armchair (`self.Armchair`))
  (bind _armchair1 (`self.Armchair1`))
  (bind _pointlight (`self.PointLight`))
  (bind _portal (`self.Portal`))
  (`PrimitiveComponent.SetCollisionEnabled` (`self.Box`) "QueryAndPhysics")
  (`|ExecutionSequence`
    (:`then_0`
      (bind (_direction _newtrack_0) (`Timeline|Timeline_0` :!via `PlayFromStart`)
        (:`Update`
          (`SceneComponent.K2_SetRelativeLocation` _armchair (`KismetMathLibrary.VLerp` (`SceneComponent.RelativeLocation` _armchair) (111.0 -1.0 0.0) _newtrack_0) false false)
          (`SceneComponent.SetRelativeScale3D` _portal (`KismetMathLibrary.VLerp` (`SceneComponent.RelativeScale3D` _portal) (0.0 0.0 0.0) _newtrack_0))
          (`LightComponent.SetIntensity` _pointlight (`KismetMathLibrary.Lerp` (`LightComponentBase.Intensity` _pointlight) 0.0 _newtrack_0)))))
    (:`then_1`
      (bind (_direction_2 _newtrack_0_2) (`Timeline|Timeline_1` :!via `PlayFromStart`)
        (:`Update`
          (`SceneComponent.K2_SetRelativeLocation` _armchair1 (`KismetMathLibrary.VLerp` (`SceneComponent.RelativeLocation` _armchair1) (-111.0 0.0 0.0) _newtrack_0_2) false false))))))

(fn `UserConstructionScript`)