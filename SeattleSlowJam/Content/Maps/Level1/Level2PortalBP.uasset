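; Level 2 portal actor in Level 1 that switches between a small state and a large, relocated state via ShrinkEvent and ExpandEvent.
; Shrink enables box collision and raises the point light intensity; Expand disables the collision.
; Each event plays its own timeline, lerping actor scale, world location and Portal component scale from their current values toward hardcoded targets.
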(event `ShrinkEvent`
  (bind _portal (`self.Portal`))
  (bind _pointlight (`self.PointLight`))
  (`PrimitiveComponent.SetCollisionEnabled` (`self.Box`) "QueryAndPhysics")
  (bind (_direction _newtrack_0) (`Timeline|Timeline_0` :!via `PlayFromStart`)
    (:`Update`
      (`self.SetActorScale3D` (`KismetMathLibrary.VLerp` (`self.GetActorScale3D`) (1.5 1.5 1.5) _newtrack_0))
      (`SceneComponent.SetRelativeScale3D` _portal (`KismetMathLibrary.VLerp` (`SceneComponent.RelativeScale3D` _portal) (1.0 0.7775 1.0) (* _newtrack_0 0.5)))
      (`self.K2_SetActorLocation` (`KismetMathLibrary.VLerp` (`self.K2_GetActorLocation`) (-490.0 13890.0 270.0) _newtrack_0))
      (`LightComponent.SetIntensity` _pointlight (`KismetMathLibrary.Lerp` (`LightComponentBase.Intensity` _pointlight) 55.0 _newtrack_0)))))

(event `ExpandEvent`
  (bind _portal (`self.Portal`))
  (`PrimitiveComponent.SetCollisionEnabled` (`self.Box`) "NoCollision")
  (bind (_direction _newtrack_0) (`Timeline|Timeline_1` :!via `PlayFromStart`)
    (:`Update`
      (`self.SetActorScale3D` (`KismetMathLibrary.VLerp` (`self.GetActorScale3D`) (4.0 9.0 4.0) _newtrack_0))
      (`self.K2_SetActorLocation` (`KismetMathLibrary.VLerp` (`self.K2_GetActorLocation`) (-490.0 37040.0 -860.0) _newtrack_0))
      (`SceneComponent.SetRelativeScale3D` _portal (`KismetMathLibrary.VLerp` (`SceneComponent.RelativeScale3D` _portal) (1.0 0.43 1.0) _newtrack_0)))))

(fn `UserConstructionScript`)