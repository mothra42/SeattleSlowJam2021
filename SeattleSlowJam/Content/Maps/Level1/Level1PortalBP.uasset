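; Level 1 portal Blueprint whose ShrinkEvent animates the portal, its two plants and a point light.
; The event enables query-and-physics collision on the Box, then starts two timelines together through a Sequence.
; One moves Plant, scales Portal to unit size and fades the light out, while the other moves Plant1 to its relative origin.
; Each update lerps from the current value, so motion compounds rather than following the curve directly.
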(event `ShrinkEvent`
  (bind _pointlight (`self.PointLight`))
  (bind _portal (`self.Portal`))
  (bind _plant (`self.Plant`))
  (bind _plant1 (`self.Plant1`))
  (`PrimitiveComponent.SetCollisionEnabled` (`self.Box`) "QueryAndPhysics")
  (`|ExecutionSequence`
    (:`then_0`
      (bind (_direction _newtrack_0) (`Timeline|Timeline_0` :!via `PlayFromStart`)
        (:`Update`
          (`SceneComponent.K2_SetRelativeLocation` _plant (`KismetMathLibrary.VLerp` (`SceneComponent.RelativeLocation` _plant) (0.0 -1.0 0.0) _newtrack_0) false false)
          (`SceneComponent.SetRelativeScale3D` _portal (`KismetMathLibrary.VLerp` (`SceneComponent.RelativeScale3D` _portal) (1.0 1.0 1.0) _newtrack_0))
          (`LightComponent.SetIntensity` _pointlight (`KismetMathLibrary.Lerp` (`LightComponentBase.Intensity` _pointlight) 0.0 _newtrack_0)))))
    (:`then_1`
      (bind (_direction_2 _newtrack_0_2) (`Timeline|Timeline_2` :!via `PlayFromStart`)
        (:`Update`
          (`SceneComponent.K2_SetRelativeLocation` _plant1 (`KismetMathLibrary.VLerp` (`SceneComponent.RelativeLocation` _plant1) (0.0 0.0 0.0) _newtrack_0_2) false false))))))

(fn `UserConstructionScript`)