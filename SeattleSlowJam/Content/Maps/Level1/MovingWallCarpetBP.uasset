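; Moving wall carpet actor for Level 1 that slides its mesh along local Y and shoves the player's cabin character on contact.
; A timeline starts on BeginPlay and alternates reverse and forward through a FlipFlop on finish.
; Each update offsets the mesh from its current location, not a stored origin, by Speed scaled by the track.
; Box hits pass the normal impulse to the character's movement and print a debug message.
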(event `self.Box.OnComponentHit`
  (params (HitComponent :type "PrimitiveComponent Object Reference") (OtherActor :type "Actor Object Reference") (OtherComp :type "PrimitiveComponent Object Reference") (NormalImpulse :type "Vector Structure") (Hit :type "HitResult Structure (by ref)"))
  (bind _ascabin_character_bp (cast `/Game/ThirdPersonCPP/Blueprints/CabinCharacter_BP` OtherActor))
  (`CharacterMovementComponent.AddImpulse` (`Character.CharacterMovement` _ascabin_character_bp) NormalImpulse false)
  (`KismetSystemLibrary.PrintString` "Hello"))

(event `self.ReceiveBeginPlay`
  (bind (_relativelocation_x _relativelocation_y _relativelocation_z) (`KismetMathLibrary.BreakVector` (`SceneComponent.RelativeLocation` (`self.ItemMesh`))))
  (`parent.ReceiveBeginPlay`)
  (bind (_direction _newtrack_0) (`Timeline|Move` :!via `PlayFromStart` :!label _label)
    (:`Update`
      (`KismetSystemLibrary.MoveComponentTo` (`self.ItemMesh`) (`KismetMathLibrary.VLerp` (`SceneComponent.RelativeLocation` (`self.ItemMesh`)) (`KismetMathLibrary.MakeVector` _relativelocation_x (+ _relativelocation_y (`self.Speed`)) _relativelocation_z) _newtrack_0) (struct) false false 0.0))
    (:`Finished`
      (`/Engine/EditorBlueprintResources/StandardMacros.FlipFlop`
        (:`A`
          (goto _label :!via `Reverse`))
        (:`B`
          (goto _label))))))

(fn `UserConstructionScript`
  (`parent.UserConstructionScript`))