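; Portal fireplace actor that switches between expanded and shrunk states through two custom events, whose callers are outside this graph.
; ShrinkEvent enables Box collision and runs a timeline moving the actor, scaling it to unit size and adjusting its PointLight.
; ExpandEvent disables collision, prints a debug string and runs a timeline enlarging FirePlace while moving the actor elsewhere.
; Both lerp from current values each update toward hardcoded world positions, compounding the easing.
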(event `ShrinkEvent`
  (bind _pointlight (`self.PointLight`))
  (`PrimitiveComponent.SetCollisionEnabled` (`self.Box`) "QueryAndPhysics")
  (bind (_direction _newtrack_0) (`Timeline|Shrink` :!via `PlayFromStart`)
    (:`Update`
      (`self.SetActorScale3D` (`KismetMathLibrary.VLerp` (`self.GetActorScale3D`) (1.0 1.0 1.0) _newtrack_0))
      (`self.K2_SetActorLocation` (`KismetMathLibrary.VLerp` (`self.K2_GetActorLocation`) (-490.0 13890.0 270.0) _newtrack_0))
      (`LightComponent.SetIntensity` _pointlight (`KismetMathLibrary.Lerp` (`LightComponentBase.Intensity` _pointlight) 55.0 _newtrack_0)))))

(event `ExpandEvent`
  (`PrimitiveComponent.SetCollisionEnabled` (`self.Box`) "NoCollision")
  (`KismetSystemLibrary.PrintString` "Hello")
  (bind (_direction _newtrack_0) (`Timeline|Expand` :!via `PlayFromStart`)
    (:`Update`
      (`SceneComponent.SetWorldScale3D` (`self.FirePlace`) (`KismetMathLibrary.VLerp` (`SceneComponent.K2_GetComponentScale` (`self.FirePlace`)) (4.0 9.0 4.0) _newtrack_0))
      (`self.K2_SetActorLocation` (`KismetMathLibrary.VLerp` (`self.K2_GetActorLocation`) (-490.0 37040.0 -860.0) _newtrack_0)))))

(fn `UserConstructionScript`)