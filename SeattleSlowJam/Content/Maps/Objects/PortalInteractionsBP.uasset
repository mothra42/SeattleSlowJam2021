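; Handles portal travel between the cabin and dungeon, auto-walking the player while input is disabled.
; Dungeon entry centers the camera by timeline, teleports, reconfigures the camera boom and streams in LevelName.
; The walk-out event unloads CabinLevel, hides the portal and restores input.
; Returning home uses a timeline as a delay, then teleports player and collected items, resets the camera, shrinks the exit portal cone and reloads CabinLevel.
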(event `WalkOutOfPortalEvent`
  (params (HideShowPortal :type "Actor Object Reference"))
  ;[1 1 1] Walk out of portal in dungeon
  (`GameplayStatics.UnloadStreamLevel` "CabinLevel")
  (`AIBlueprintHelperLibrary.SimpleMoveToLocation` (`GameplayStatics.GetPlayerController` 0) (-486.845612 14285.075195 328.6987))
  (`KismetSystemLibrary.Delay` 0.9)
  (`self.SetActorHiddenInGame` HideShowPortal true)
  (bind _ascabin_character_bp (cast `/Game/ThirdPersonCPP/Blueprints/CabinCharacter_BP` (`GameplayStatics.GetPlayerPawn` 0)))
  (`self.EnableInput` _ascabin_character_bp (`GameplayStatics.GetPlayerController` 0)))

(event `TeleportHomeEvent`
  (params (Actor :type "Actor Object Reference"))
  (bind _returnvalue (`GameplayStatics.GetPlayerController` 0))
  (bind _returnvalue_2 (`GameplayStatics.GetPlayerController` 0))
  (bind _as_cabin_character_bp (`self.As Cabin Character BP`))
  ;[1 1 1] Teleport home
  (bind _ascabin_character_bp (cast `/Game/ThirdPersonCPP/Blueprints/CabinCharacter_BP` (`GameplayStatics.GetPlayerPawn` 0)))
  (bind _output_get (set `self.As Cabin Character BP` _ascabin_character_bp))
  (`AIBlueprintHelperLibrary.SimpleMoveToActor` _returnvalue_2 Actor)
  (`CabinCharacter.ShouldConstrainMovement` _as_cabin_character_bp false)
  (`self.DisableInput` _as_cabin_character_bp _returnvalue_2)
  (`Controller.SetIgnoreLookInput` _returnvalue_2 false)
  (`Timeline|Delay because real delay doesn't work` :!via `PlayFromStart`
    (:`Finished`
      (`self.K2_TeleportTo` _output_get (840.0 330.0 -622.0) (struct :`Yaw` 270.0))
      (bind _returnvalue_3 (`GameplayStatics.GetActorOfClass` "/Script/SeattleSlowJam.ItemTeleportationArea"))
      (`ItemTeleportationArea.TeleportAllCollectedItems` _returnvalue_3)
      (set `SpringArmComponent.TargetArmLength` 348.519165 (`CabinCharacter.CameraBoom` (`self.As Cabin Character BP`)))
      (set `SpringArmComponent.bDoCollisionTest` true (`CabinCharacter.CameraBoom` (`self.As Cabin Character BP`)))
      (`Controller.SetControlRotation` _returnvalue (`KismetMathLibrary.MakeRotator` 0.0 355.0 270.0))
      (`NavMovementComponent.StopActiveMovement` (`Character.CharacterMovement` (`self.As Cabin Character BP`)))
      (`SceneComponent.K2_SetRelativeLocation` (`CabinCharacter.CameraBoom` (`self.As Cabin Character BP`)) (0.0 0.0 0.0) false false)
      (bind _outactors (`GameplayStatics.GetAllActorsOfClass` "/Game/Maps/Objects/CabinExitPortal.CabinExitPortal_C"))
      (`/Game/Maps/Objects/CabinExitPortal.ConeShrinkEvent` (`|GetArrayItem` _outactors))
      (`GameplayStatics.LoadStreamLevel` "CabinLevel" true)
      (`KismetSystemLibrary.Delay` 1.0)
      (`self.EnableInput` (`self.As Cabin Character BP`) _returnvalue))))

(event `AutoWalkAndTPToDungeonEvent`
  (params (WalkTo :type "Actor Object Reference") (`TeleportPoint ` :type "Actor Object Reference"))
  (bind _returnvalue (`GameplayStatics.GetPlayerController` 0))
  (bind _as_cabin_character_bp (`self.As Cabin Character BP`))
  (bind (_returnvalue_roll _returnvalue_pitch _returnvalue_yaw) (`KismetMathLibrary.BreakRotator` (`Controller.GetControlRotation` _returnvalue)))
  (bind _cameraboom (`CabinCharacter.CameraBoom` _as_cabin_character_bp))
  ;[1 1 1] Teleport to dungeon
  (bind _ascabin_character_bp (cast `/Game/ThirdPersonCPP/Blueprints/CabinCharacter_BP` (`GameplayStatics.GetPlayerPawn` 0)))
  (bind _output_get (set `self.As Cabin Character BP` _ascabin_character_bp))
  (`CabinCharacter.ShouldConstrainMovement` _output_get true)
  (`self.DisableInput` _output_get _returnvalue)
  (`Controller.SetIgnoreLookInput` _returnvalue true)
  (`AIBlueprintHelperLibrary.SimpleMoveToActor` _returnvalue WalkTo)
  (bind (_direction _newtrack_0) (`Timeline|Center Camera ToPortal Timeline` :!via `PlayFromStart`)
    (:`Update`
      (`Controller.SetControlRotation` _returnvalue (`KismetMathLibrary.MakeRotator` 0.0 (`KismetMathLibrary.Lerp` _returnvalue_pitch (`KismetMathLibrary.FClamp` (`KismetMathLibrary.SelectFloat` (- _returnvalue_pitch 11.0) (+ _returnvalue_pitch 11.0) (`KismetMathLibrary.InRange_FloatFloat` _returnvalue_pitch 1.0 100.0)) 0.0 355.0) _newtrack_0) (`KismetMathLibrary.Lerp` _returnvalue_yaw 90.0 _newtrack_0))))
    (:`Finished`
      (`Controller.SetControlRotation` (`GameplayStatics.GetPlayerController` 0) (`KismetMathLibrary.MakeRotator` 0.0))
      (`self.K2_TeleportTo` _as_cabin_character_bp (`self.K2_GetActorLocation` `TeleportPoint `) (struct :`Yaw` 90.0))
      (set `SpringArmComponent.TargetArmLength` 700.0 _cameraboom)
      (`SceneComponent.K2_SetRelativeLocation` _cameraboom (0.0 0.0 111.0) false false)
      (set `SpringArmComponent.bDoCollisionTest` false (`CabinCharacter.CameraBoom` (`self.As Cabin Character BP`)))
      (`GameplayStatics.LoadStreamLevel` (`self.Level Name`) true))))

(fn `UserConstructionScript`)